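; Player controller for a tile-board game with mine marking, turning input into board updates and character movement.
; BeginPlay caches the first BoardView and DemoCharacter actors in the level.
; SetDestination updates the tile under the cursor and moves the player there, while MarkMine flags it, both gated by DoOnce until release.
; WhatDidWeHit casts the cursor trace hit to TileBase, returning its grid coordinates and world location with debug prints.
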(event EventBeginPlay
  (Utilities|FlowControl|Sequence
    (:then_0
      (bind _outactors (Actor|GetAllActorsOfClass "/Game/Board/Blueprints/BoardView.BoardView_C"))
      (Variables|Default|SetBoardView (Utilities|Array|Get(acopy) _outactors)))
    (:then_1
      (bind _outactors_2 (Actor|GetAllActorsOfClass "/Game/2DCharacter/Characters/DemoCharacter.DemoCharacter_C"))
      (Variables|Default|Setourplayer (Utilities|Array|Get(acopy) _outactors_2)))))

(event EventTick
  (params (DeltaSeconds :type Float%20%28single-precision%29)))

(event Input|ActionEvents|InputActionSetDestination
  (params (Key :type Key%20Structure))
  (:Pressed
    (Utilities|FlowControl|DoOnce false :!label _label
      (:Completed
        (bind (_x _y _location_in_world) (CallFunction|WhatDidWeHit (.HitResult (Game|Player|GetHitResultUnderCursorbyChannel "TraceTypeQuery1" true))))
        (Default|UpdateBoard (Variables|Default|GetBoardView) _x _y)
        (Default|MovetoAction (Variables|Default|Getourplayer) _location_in_world))))
  (:Released
    (goto _label Reset)))

(event Input|ActionEvents|InputActionMarkMine
  (params (Key :type Key%20Structure))
  (:Pressed
    (Utilities|FlowControl|DoOnce false :!label _label
      (:Completed
        (bind (_x _y) (CallFunction|WhatDidWeHit (.HitResult (Game|Player|GetHitResultUnderCursorbyChannel "TraceTypeQuery1" true))))
        (Default|MarkMine (Variables|Default|GetBoardView) _x _y))))
  (:Released
    (goto _label Reset)))

(fn ConstructionScript)

(fn WhatDidWeHit
  (params (hit :type Hit%20Result%20Structure))
  (bind _hitactor (Collision|BreakHitResult hit))
  (bind _output_get (Variables|Default|SetHitActor _hitactor))
  (Utilities|Casting|CastToTileBaseClass (Utilities|GetClass _hitactor))
  (bind _astile_base (Utilities|Casting|CastToTileBase _output_get))
  (Development|PrintString "You have selected Tile with")
  (Development|PrintString (Utilities|String|ToString(Integer) (Variables|/Game/Board/Blueprints/Tiles/TileBase.TileBase_C|GetX _astile_base)))
  (Development|PrintString (Utilities|String|ToString(Integer) (Variables|/Game/Board/Blueprints/Tiles/TileBase.TileBase_C|GetY _astile_base)))
  (return (Variables|/Game/Board/Blueprints/Tiles/TileBase.TileBase_C|GetX _astile_base) (Variables|/Game/Board/Blueprints/Tiles/TileBase.TileBase_C|GetY _astile_base) (.location (Transformation|GetActorTransform _astile_base))))