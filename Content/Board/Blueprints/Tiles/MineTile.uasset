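; MineTile is a board tile Blueprint that shows a hidden or revealed sprite for a mine tile.
; UpdateSprite reads IsHidden from the given TileModel and sets the Paper2D sprite to match.
; Hidden tiles use HiddenSprite when it is valid and fall back to DefaultHiddenSprite otherwise, while revealed tiles use RevealedSprite.
; The event graph holds only disabled stubs, and the construction script just calls its parent.
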(event EventBeginPlay
  (|CallParentFunction) ; This node is disabled and will not be called.\nDrag off pins to build functionality.
)

(event Collision|EventActorBeginOverlap
  (params (OtherActor :type Actor%20Object%20Reference))
  (|CallParentFunction OtherActor) ; This node is disabled and will not be called.\nDrag off pins to build functionality.
)

(event EventTick
  (params (DeltaSeconds :type Float%20%28single-precision%29))
  (|CallParentFunction DeltaSeconds) ; This node is disabled and will not be called.\nDrag off pins to build functionality.
)

(fn ConstructionScript
  (|CallParentFunction))

(fn UpdateSprite
  (params (TileModel :type Tile%20Model%20Structure))
  (if (.isHidden (Utilities|Struct|BreakTileModel TileModel))
    (Utilities|IsValid (Variables|Default|GetHiddenSprite)
      (:Is%20Valid
        (Rendering|Components|Sprite|SetSprite (Variables|Default|GetPaperSprite) (Variables|Default|GetHiddenSprite)))
      (:Is%20Not%20Valid
        (Rendering|Components|Sprite|SetSprite (Variables|Default|GetPaperSprite) (Variables|Default|GetDefaultHiddenSprite))))
    (else
      (Rendering|Components|Sprite|SetSprite (Variables|Default|GetPaperSprite) (Variables|Sprites|GetRevealedSprite))))
  (return self))