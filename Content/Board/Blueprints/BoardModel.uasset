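; BoardModel holds the state and rules of a Minesweeper game as a 2D grid of tile structs.
; BuildBoard creates the tiles, places random mines through recursive, attempt-capped MakeMines, then stores each tile's neighboring mine count.
; MoveToMine calls Reveal, a recursive flood fill that threads a visited-coordinate map through empty neighbors and flags a loss on a directly revealed mine.
; ToggleMarkedMine flips marks, and CheckForWin declares victory once every mine is marked.
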(event EventBeginPlay)

(event Collision|EventActorBeginOverlap
  (params (OtherActor :type Actor%20Object%20Reference)))

(event EventTick
  (params (DeltaSeconds :type Float%20%28single-precision%29)))

(fn ConstructionScript)

(fn BuildBoard
  (bind _width (Variables|Default|GetWidth))
  (bind _height (Variables|Default|GetHeight))
  (bind _numberofmines (Variables|Default|GetNumberOfMines))
  ;[1 1 1] Init Tiles
  (Utilities|Array|Resize (Variables|Default|GetTiles) _height)
  (for _index (range 0 (- _height 1))
    (Utilities|Array|Resize (Utilities|Struct|BreakTileArray (Utilities|Array|Get(acopy) (Variables|Default|GetTiles) _index)) _width)
    (for _index_2 (range 0 (- _width 1))
      (CallFunction|SetTile _index_2 _index (Utilities|Struct|MakeTileModel true false 0 _index_2 _index))))
  ;[1 1 1] Add Mines
  (CallFunction|MakeMines _numberofmines 0 (* _numberofmines 2))
  ;[1 1 1] Update Number of Tiles Touching
  (for (_array_element _array_index) (Variables|Default|GetTiles)
    (for (_ _array_index_2) (Utilities|Struct|BreakTileArray _array_element)
      (CallFunction|SetNumberOfMinesTouching (Utilities|GetTile _array_index _array_index_2))))
  (return))

(fn MakeMines
  (params (minesToMake :type Integer) (attempts :type Integer) (maxAttempts :type Integer))
  (bind _returnvalue (- minesToMake 1))
  (bind _returnvalue_2 (+ attempts 1))
  (bind _tile (Utilities|GetRandomTile))
  (bind (_ishidden _ismarked _numberofminestouching _x _y _type) (Utilities|Struct|BreakTileModel _tile))
  (if (> attempts maxAttempts)
    (return)
    (else
      (if (Utilities|Enum|Equal(Enum) _type "NewEnumerator1")
        (CallFunction|MakeMines minesToMake _returnvalue_2 maxAttempts)
        (else
          (CallFunction|SetTile _x _y (Utilities|Struct|MakeTileModel true false 0 _x _y "NewEnumerator1"))
          (if (> _returnvalue 0)
            (CallFunction|MakeMines _returnvalue _returnvalue_2 maxAttempts))))
      (return))))

(fn SetTile
  (params (X :type Integer) (Y :type Integer) (Tile :type Tile%20Model%20Structure))
  (Utilities|Array|SetArrayElem (Utilities|Struct|BreakTileArray (Utilities|Array|Get(acopy) (Variables|Default|GetTiles) Y)) X Tile)
  (return))

(fn SetNumberOfMinesTouching
  (params (Tile :type Tile%20Model%20Structure))
  (LocalVariables|SetTileToTest Tile)
  ;[1 1 1] Top-Left
  (bind _isvalidcoord (CallFunction|IsValidCoord (- (.x (Utilities|Struct|BreakTileModel (LocalVariables|GetTileToTest))) 1) (- (.y (Utilities|Struct|BreakTileModel (LocalVariables|GetTileToTest))) 1)))
  (if (and _isvalidcoord (Utilities|Enum|Equal(Enum) (.type (Utilities|Struct|BreakTileModel (Utilities|GetTile (- (.y (Utilities|Struct|BreakTileModel (LocalVariables|GetTileToTest))) 1) (- (.x (Utilities|Struct|BreakTileModel (LocalVariables|GetTileToTest))) 1)))) "NewEnumerator1"))
    (Math|Integer|IncrementInt (LocalVariables|GetNumberTouchinng)
      (:%20%20
        _)))
  ;[1 1 1] Top
  (bind _isvalidcoord_2 (CallFunction|IsValidCoord (.x (Utilities|Struct|BreakTileModel (LocalVariables|GetTileToTest))) (- (.y (Utilities|Struct|BreakTileModel (LocalVariables|GetTileToTest))) 1)))
  (if (and _isvalidcoord_2 (Utilities|Enum|Equal(Enum) (.type (Utilities|Struct|BreakTileModel (Utilities|GetTile (- (.y (Utilities|Struct|BreakTileModel (LocalVariables|GetTileToTest))) 1) (.x (Utilities|Struct|BreakTileModel (LocalVariables|GetTileToTest)))))) "NewEnumerator1"))
    (Math|Integer|IncrementInt (LocalVariables|GetNumberTouchinng)
      (:%20%20
        _)))
  ;[1 1 1] Top-Right
  (bind _isvalidcoord_3 (CallFunction|IsValidCoord (+ (.x (Utilities|Struct|BreakTileModel (LocalVariables|GetTileToTest))) 1) (- (.y (Utilities|Struct|BreakTileModel (LocalVariables|GetTileToTest))) 1)))
  (if (and _isvalidcoord_3 (Utilities|Enum|Equal(Enum) (.type (Utilities|Struct|BreakTileModel (Utilities|GetTile (- (.y (Utilities|Struct|BreakTileModel (LocalVariables|GetTileToTest))) 1) (+ (.x (Utilities|Struct|BreakTileModel (LocalVariables|GetTileToTest))) 1)))) "NewEnumerator1"))
    (Math|Integer|IncrementInt (LocalVariables|GetNumberTouchinng)
      (:%20%20
        _)))
  ;[1 1 1] Middle-Left
  (bind _isvalidcoord_4 (CallFunction|IsValidCoord (- (.x (Utilities|Struct|BreakTileModel (LocalVariables|GetTileToTest))) 1) (.y (Utilities|Struct|BreakTileModel (LocalVariables|GetTileToTest)))))
  (if (and _isvalidcoord_4 (Utilities|Enum|Equal(Enum) (.type (Utilities|Struct|BreakTileModel (Utilities|GetTile (.y (Utilities|Struct|BreakTileModel (LocalVariables|GetTileToTest))) (- (.x (Utilities|Struct|BreakTileModel (LocalVariables|GetTileToTest))) 1)))) "NewEnumerator1"))
    (Math|Integer|IncrementInt (LocalVariables|GetNumberTouchinng)
      (:%20%20
        _)))
  ;[1 1 1] Middle-Right
  (bind _isvalidcoord_5 (CallFunction|IsValidCoord (+ (.x (Utilities|Struct|BreakTileModel (LocalVariables|GetTileToTest))) 1) (.y (Utilities|Struct|BreakTileModel (LocalVariables|GetTileToTest)))))
  (if (and _isvalidcoord_5 (Utilities|Enum|Equal(Enum) (.type (Utilities|Struct|BreakTileModel (Utilities|GetTile (.y (Utilities|Struct|BreakTileModel (LocalVariables|GetTileToTest))) (+ (.x (Utilities|Struct|BreakTileModel (LocalVariables|GetTileToTest))) 1)))) "NewEnumerator1"))
    (Math|Integer|IncrementInt (LocalVariables|GetNumberTouchinng)
      (:%20%20
        _)))
  ;[1 1 1] Bottom-Left
  (bind _isvalidcoord_6 (CallFunction|IsValidCoord (- (.x (Utilities|Struct|BreakTileModel (LocalVariables|GetTileToTest))) 1) (+ (.y (Utilities|Struct|BreakTileModel (LocalVariables|GetTileToTest))) 1)))
  (if (and _isvalidcoord_6 (Utilities|Enum|Equal(Enum) (.type (Utilities|Struct|BreakTileModel (Utilities|GetTile (+ (.y (Utilities|Struct|BreakTileModel (LocalVariables|GetTileToTest))) 1) (- (.x (Utilities|Struct|BreakTileModel (LocalVariables|GetTileToTest))) 1)))) "NewEnumerator1"))
    (Math|Integer|IncrementInt (LocalVariables|GetNumberTouchinng)
      (:%20%20
        _)))
  ;[1 1 1] Bottom
  (bind _isvalidcoord_7 (CallFunction|IsValidCoord (.x (Utilities|Struct|BreakTileModel (LocalVariables|GetTileToTest))) (+ (.y (Utilities|Struct|BreakTileModel (LocalVariables|GetTileToTest))) 1)))
  (if (and _isvalidcoord_7 (Utilities|Enum|Equal(Enum) (.type (Utilities|Struct|BreakTileModel (Utilities|GetTile (+ (.y (Utilities|Struct|BreakTileModel (LocalVariables|GetTileToTest))) 1) (.x (Utilities|Struct|BreakTileModel (LocalVariables|GetTileToTest)))))) "NewEnumerator1"))
    (Math|Integer|IncrementInt (LocalVariables|GetNumberTouchinng)
      (:%20%20
        _)))
  ;[1 1 1] Bottom-Right
  (bind _isvalidcoord_8 (CallFunction|IsValidCoord (+ (.x (Utilities|Struct|BreakTileModel (LocalVariables|GetTileToTest))) 1) (+ (.y (Utilities|Struct|BreakTileModel (LocalVariables|GetTileToTest))) 1)))
  (if (and _isvalidcoord_8 (Utilities|Enum|Equal(Enum) (.type (Utilities|Struct|BreakTileModel (Utilities|GetTile (+ (.y (Utilities|Struct|BreakTileModel (LocalVariables|GetTileToTest))) 1) (+ (.x (Utilities|Struct|BreakTileModel (LocalVariables|GetTileToTest))) 1)))) "NewEnumerator1"))
    (Math|Integer|IncrementInt (LocalVariables|GetNumberTouchinng)
      (:%20%20
        _)))
  ;[1 1 1] Update Tile
  (CallFunction|SetTile (.x (Utilities|Struct|BreakTileModel (LocalVariables|GetTileToTest))) (.y (Utilities|Struct|BreakTileModel (LocalVariables|GetTileToTest))) (Utilities|Struct|MakeTileModel (.isHidden (Utilities|Struct|BreakTileModel (LocalVariables|GetTileToTest))) false (LocalVariables|GetNumberTouchinng) (.x (Utilities|Struct|BreakTileModel (LocalVariables|GetTileToTest))) (.y (Utilities|Struct|BreakTileModel (LocalVariables|GetTileToTest))) (.type (Utilities|Struct|BreakTileModel (LocalVariables|GetTileToTest)))))
  (return))

(fn IsValidCoord
  (params (x :type Integer) (y :type Integer))
  (return (Math|Boolean|ANDBoolean (>= x 0) (< x (Variables|Default|GetWidth)) (>= y 0) (< y (Variables|Default|GetHeight)))))

(fn Reveal
  (params (X :type Integer) (Y :type Integer) (revealMines :type Boolean) (coordsVisited :type Map%20of%20Vector%202D%20Structures%20to%20Booleans))
  (if (Utilities|HasEnded)
    (return 0)
    (else
      (LocalVariables|SettempTilesVisited coordsVisited)
      (LocalVariables|SettileX X)
      (LocalVariables|SettileY Y)
      (LocalVariables|SetshouldRevealMine revealMines)
      (bind _isvalidcoord (CallFunction|IsValidCoord (LocalVariables|GettileX) (LocalVariables|GettileY)))
      (if _isvalidcoord
        (LocalVariables|Settile (Utilities|GetTile (LocalVariables|GettileY) (LocalVariables|GettileX)))
        (if (and (.Value (Utilities|Map|Find (LocalVariables|GettempTilesVisited) (Math|Vector2D|MakeVector2D (Math|Conversions|ToFloat(Integer) (LocalVariables|GettileX)) (Math|Conversions|ToFloat(Integer) (LocalVariables|GettileY))))) (.ReturnValue (Utilities|Map|Find (LocalVariables|GettempTilesVisited) (Math|Vector2D|MakeVector2D (Math|Conversions|ToFloat(Integer) (LocalVariables|GettileX)) (Math|Conversions|ToFloat(Integer) (LocalVariables|GettileY))))))
          (return (LocalVariables|GettempTilesVisited))
          (else
            (Utilities|Map|Add (LocalVariables|GettempTilesVisited) (Math|Vector2D|MakeVector2D (Math|Conversions|ToFloat(Integer) (LocalVariables|GettileX)) (Math|Conversions|ToFloat(Integer) (LocalVariables|GettileY))) true)
            (if (not (.isHidden (Utilities|Struct|BreakTileModel (LocalVariables|Gettile))))
              (return (LocalVariables|GettempTilesVisited))
              (elif (Utilities|Enum|Equal(Enum) (.type (Utilities|Struct|BreakTileModel (LocalVariables|Gettile))) "NewEnumerator1")
                (if (LocalVariables|GetshouldRevealMine)
                  (CallFunction|SetTile (LocalVariables|GettileX) (LocalVariables|GettileY) (Utilities|Struct|MakeTileModel false false (.numberOfMinesTouching (Utilities|Struct|BreakTileModel (LocalVariables|Gettile))) (.x (Utilities|Struct|BreakTileModel (LocalVariables|Gettile))) (.y (Utilities|Struct|BreakTileModel (LocalVariables|Gettile))) (.type (Utilities|Struct|BreakTileModel (LocalVariables|Gettile)))))
                  (Variables|Default|SetHasLost true)
                  (return (LocalVariables|GettempTilesVisited))
                  (else
                    (return (LocalVariables|GettempTilesVisited))))
                (else
                  (CallFunction|SetTile (LocalVariables|GettileX) (LocalVariables|GettileY) (Utilities|Struct|MakeTileModel false false (.numberOfMinesTouching (Utilities|Struct|BreakTileModel (LocalVariables|Gettile))) (.x (Utilities|Struct|BreakTileModel (LocalVariables|Gettile))) (.y (Utilities|Struct|BreakTileModel (LocalVariables|Gettile))) (.type (Utilities|Struct|BreakTileModel (LocalVariables|Gettile)))))
                  (if (or (> (.numberOfMinesTouching (Utilities|Struct|BreakTileModel (LocalVariables|Gettile))) 0) (Utilities|Enum|Equal(Enum) (.type (Utilities|Struct|BreakTileModel (LocalVariables|Gettile))) "NewEnumerator1"))
                    (return (LocalVariables|GettempTilesVisited))
                    (else
                      (bind _updatedtilesvisited (CallFunction|Reveal (- (LocalVariables|GettileX) 1) (- (LocalVariables|GettileY) 1) false (LocalVariables|GettempTilesVisited)))
                      (bind _updatedtilesvisited_2 (CallFunction|Reveal (LocalVariables|GettileX) (- (LocalVariables|GettileY) 1) false _updatedtilesvisited))
                      (bind _updatedtilesvisited_3 (CallFunction|Reveal (+ (LocalVariables|GettileX) 1) (- (LocalVariables|GettileY) 1) false _updatedtilesvisited_2))
                      (bind _updatedtilesvisited_4 (CallFunction|Reveal (- (LocalVariables|GettileX) 1) (LocalVariables|GettileY) false _updatedtilesvisited_3))
                      (bind _updatedtilesvisited_5 (CallFunction|Reveal (+ (LocalVariables|GettileX) 1) (LocalVariables|GettileY) false _updatedtilesvisited_4))
                      (bind _updatedtilesvisited_6 (CallFunction|Reveal (- (LocalVariables|GettileX) 1) (+ (LocalVariables|GettileY) 1) false _updatedtilesvisited_5))
                      (bind _updatedtilesvisited_7 (CallFunction|Reveal (LocalVariables|GettileX) (+ (LocalVariables|GettileY) 1) false _updatedtilesvisited_6))
                      (bind _updatedtilesvisited_8 (CallFunction|Reveal (+ (LocalVariables|GettileX) 1) (+ (LocalVariables|GettileY) 1) false _updatedtilesvisited_7))
                      (return _updatedtilesvisited_8))))))))
        (else
          (return (LocalVariables|GettempTilesVisited)))))))

(fn CheckforWin
  (for _array_element (Variables|Default|GetTiles)
    (for _array_element_2 (Utilities|Struct|BreakTileArray _array_element)
      (if (Utilities|Enum|Equal(Enum) (.type (Utilities|Struct|BreakTileModel _array_element_2)) "NewEnumerator1")
        (if (not (.isMarked (Utilities|Struct|BreakTileModel _array_element_2)))
          ;[1 1 1] Found an unmarked mine
          (Variables|Default|SetHasWon false)
          (return)))))
  ;[1 1 1] All mines marked
  (Variables|Default|SetHasWon true)
  (return))

(fn MovetoMine
  (params (X :type Integer) (Y :type Integer))
  ;[1 1 1] Don't reveal if player has won or loss
  (if (not (or (Variables|Default|GetHasWon) (Variables|Default|GetHasLost)))
    (CallFunction|Reveal X Y true (Utilities|Map|MakeMap "" false))
    (CallFunction|CheckforWin)))

(fn ToggleMarkedMine
  (params (x :type Integer) (y :type Integer))
  (bind _tile (Utilities|GetTile x y))
  (bind (_ishidden _ismarked _numberofminestouching _x _y _type) (Utilities|Struct|BreakTileModel _tile))
  (CallFunction|SetTile x y (Utilities|Struct|MakeTileModel _ishidden (not _ismarked) _numberofminestouching _x _y _type))
  (CallFunction|CheckforWin))